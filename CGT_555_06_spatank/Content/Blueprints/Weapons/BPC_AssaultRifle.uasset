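; Assault rifle weapon Blueprint that fires hitscan traces and sends damage messages.
; WeaponTrace finds a camera aim point, then sphere-traces from the Arrow component toward it, though the component-wise multiply keeps only the direction's X axis.
; Hit actors implementing BPi_Damage receive Points, a counter that rises with consecutive hits and resets on any other result.
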(event EventBeginPlay
  (|CallParentFunction) ; This node is disabled and will not be called.\nDrag off pins to build functionality.
)

(event EventWeaponTrace
  (bind _arrow (Variables|Default|GetArrow))
  (bind _returnvalue (Transformation|GetWorldLocation _arrow))
  (bind _outhit (CallFunction|CameraTrace "8000.000000,5000.000000,5000.000000" 1.0 "ForDuration"))
  (bind _outhit_2 (Collision|SphereTraceByChannel _returnvalue (+ (* (Math|Vector|GetForwardVector (Math|Rotator|FindLookatRotation _returnvalue (.ImpactPoint (Collision|BreakHitResult _outhit)))) "8000.000000,0,0") _returnvalue) 1.0 "TraceTypeQuery1" false 0 "None"))
  (if (Utilities|DoesObjectImplementInterface (.HitActor (Collision|BreakHitResult _outhit_2)) "/Game/Blueprints/Weapons/BPi_Damage.BPi_Damage_C")
    (bind _output_get (Variables|Default|SetPoints (+ (Variables|Default|GetPoints) 1)))
    (Class|BPiDamage|RecieveDamage(Message) (.HitActor (Collision|BreakHitResult _outhit_2)) _output_get)
    (else
      (Variables|Default|SetPoints 0))))

(fn ConstructionScript
  (|CallParentFunction))