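; BP_WeaponBase is a weapon base Blueprint handling magazine ammo, firing effects and reloading, with an empty WeaponTrace event as a hook.
; FireWeapon checks ammo, then either reloads or updates ammo, plays muzzle particles and sound at the Arrow, traces and rechecks for reload, though the subtraction shown is zero.
; ReloadWeapon and Reload share a chain that shows an animated WB_ReloadBar, waits ReloadTime and refills the magazine.
; GetFOVMultiplier exposes the weapon's FOV multiplier.
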(event Custom|ReloadWeapon
  (bind _returnvalue (UserInterface|CreateWidget "/Game/Blueprints/Weapons/WB_ReloadBar.WB_ReloadBar_C"))
  (Default|ReloadAnimation _returnvalue (Variables|Default|GetReloadTime))
  (UserInterface|Viewport|AddtoViewport _returnvalue 0)
  (Utilities|FlowControl|Delay (Variables|Default|GetReloadTime))
  (Variables|Ammo|SetAmmo (Variables|Ammo|GetMaxMagazineAmmo)))

(event Custom|WeaponTrace)

(event EventReload
  (bind _returnvalue (UserInterface|CreateWidget "/Game/Blueprints/Weapons/WB_ReloadBar.WB_ReloadBar_C"))
  (Default|ReloadAnimation _returnvalue (Variables|Default|GetReloadTime))
  (UserInterface|Viewport|AddtoViewport _returnvalue 0)
  (Utilities|FlowControl|Delay (Variables|Default|GetReloadTime))
  (Variables|Ammo|SetAmmo (Variables|Ammo|GetMaxMagazineAmmo)))

(event EventFireWeapon
  (Utilities|INT<=INT (Variables|Ammo|GetAmmo)
    (:True
      (CallFunction|ReloadWeapon))
    (:False
      (Variables|Ammo|SetAmmo (- (Variables|Ammo|GetAmmo) 0))
      (CallFunction|WeaponFireEffects)
      (CallFunction|WeaponTrace)
      (Utilities|INT<=INT (Variables|Ammo|GetAmmo)
        (:True
          (CallFunction|ReloadWeapon))))))

(event EventBeginPlay
  (Variables|Ammo|SetAmmo (Variables|Ammo|GetMaxMagazineAmmo)))

(fn ConstructionScript)

(fn WeaponFireEffects
  (bind _arrow (Variables|Default|GetArrow))
  (bind _returnvalue (Transformation|GetWorldTransform _arrow))
  (Effects|SpawnEmitteratLocation (Variables|WeaponFireEffects|GetEmitter%20Template) (.location _returnvalue) (.rotation _returnvalue) (Variables|WeaponFireEffects|GetWeaponFireEmitterScale))
  (Audio|SpawnSoundatLocation (Variables|WeaponFireEffects|GetWeaponFireSound) (.location _returnvalue) "0, 0, 0" 1.0 1.0 0.0 0 0)
  (return))

(fn GetFOVMultiplier
  (return (Variables|Default|GetFOVMultiplier)))